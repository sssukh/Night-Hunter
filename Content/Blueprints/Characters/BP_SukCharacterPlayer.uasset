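; BP_SukCharacterPlayer is the player character Blueprint that creates the HUD and handles toggling the inventory menu.
; On BeginPlay it creates the HUD widget from the class on SukPlayerController, stores it and adds it to the viewport.
; When the HUD's ActivateInventory flag is set, IA_OpenInventory uses a FlipFlop to show or hide the inventory overlay, switching input mode and mouse cursor to match.
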(event Input|EnhancedActionEvents|EnhancedInputActionIA_OpenInventory
  (params (ActionValue :type Boolean) (ElapsedSeconds :type Float%20%28double-precision%29) (TriggeredSeconds :type Float%20%28double-precision%29) (InputAction :type Input%20Action%20Object%20Reference :default "/Game/Input/Actions/IA_OpenInventory.IA_OpenInventory"))
  (bind _bp_sukhudref (Variables|Default|GetBP_SukHUDRef))
  (bind _inventorymenuoverlay (Variables|/Game/UI/WBP_SukHUDWidget.WBP_SukHUDWidget_C|GetInventoryMenuOverlay _bp_sukhudref))
  ;[1 1 1] Toggle Inventory Menu
  (:Triggered
    (if (Variables|/Game/UI/WBP_SukHUDWidget.WBP_SukHUDWidget_C|GetActivateInventory _bp_sukhudref)
      (Utilities|FlowControl|FlipFlop
        (:A
          (Widget|SetVisibility _inventorymenuoverlay "Visible")
          (CallFunction|EnableMouseCursur))
        (:B
          (Widget|SetVisibility _inventorymenuoverlay "Hidden")
          (CallFunction|DisableMouseCursur))))))

(event EventBeginPlay
  (bind _assuk_player_controller (Utilities|Casting|CastToSukPlayerController (Pawn|GetController)))
  (bind _returnvalue (UserInterface|CreateWidget (Variables|/Script/SukProject.SukPlayerController|GetSukHUDWidgetClass _assuk_player_controller)))
  (bind _aswbp_suk_hudwidget (Utilities|Casting|CastToWBP_SukHUDWidget _returnvalue))
  (bind _output_get (Variables|Default|SetBP_SukHUDRef _aswbp_suk_hudwidget))
  (UserInterface|Viewport|AddtoViewport _output_get 0))

(event Collision|EventActorBeginOverlap
  (params (OtherActor :type Actor%20Object%20Reference)))

(event EventTick
  (params (DeltaSeconds :type Float%20%28single-precision%29)))

(fn ConstructionScript)

(fn EnableMouseCursur
  (bind _returnvalue (Game|GetPlayerController 0))
  (Input|SetInputModeGameandUI _returnvalue (Variables|Default|GetBP_SukHUDRef) "DoNotLock" true false)
  (Variables|/Script/Engine.PlayerController|SetbShowMouseCursor _returnvalue true))

(fn DisableMouseCursur
  (bind _returnvalue (Game|GetPlayerController 0))
  (Input|SetInputModeGameOnly _returnvalue false)
  (Variables|/Script/Engine.PlayerController|SetbShowMouseCursor _returnvalue false))