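; BP_TemplatePickup is a template item pickup actor whose only active logic spins its static mesh slightly around the vertical axis every Tick.
; BeginPlay, both InteractionComponent overlap events, Interaction and the construction script are empty.
; Disconnected nodes remain for an interaction text widget, in-range tracking of SukCharacterPlayer, setting the mesh from Itemcpp, and adding the item to inventory before destroying the actor, but none of them run.
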(event OnComponentBeginOverlap(InteractionComponent)
  (params (OverlappedComponent :type Primitive%20Component%20Object%20Reference) (OtherActor :type Actor%20Object%20Reference) (OtherComp :type Primitive%20Component%20Object%20Reference) (OtherBodyIndex :type Integer) (bFromSweep :type Boolean) (SweepResult :type Hit%20Result%20Structure%20%28by%20ref%29))
  ;[1 1 1] Overlap Trigger Script
)

(event OnComponentEndOverlap(InteractionComponent)
  (params (OverlappedComponent :type Primitive%20Component%20Object%20Reference) (OtherActor :type Actor%20Object%20Reference) (OtherComp :type Primitive%20Component%20Object%20Reference) (OtherBodyIndex :type Integer))
  ;[1 1 1] Overlap Trigger Script
)

(event EventTick
  (params (DeltaSeconds :type Float%20%28single-precision%29))
  (Transformation|AddWorldRotation (Variables|Default|GetStaticMesh) "0.000000,1.000000,0.000000" false false))

(event EventInteraction
  ;[1 1 1] Get Inventory Through PlayerController and
  ; Add Item Into it.
  ; And Remove this Actor.
)

(event EventBeginPlay
  ;[1 1 1] Event Begin Play
)

(fn ConstructionScript)