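; BP_SukItemPickup is an item pickup actor that takes its look and interaction prompt from its Itemcpp item.
; On BeginPlay it writes the item's InteractText into the InteractionComponent's WBP_InteractionWidget, then applies the item's mesh, both only if the widget cast succeeds.
; Tick spins the mesh by a fixed step each frame, unscaled by delta time, and the graph holds no pickup logic.
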(event EventBeginPlay
  (bind _itemcpp (Variables|Default|GetItemcpp))
  (bind _aswbp_interaction_widget (Utilities|Casting|CastToWBP_InteractionWidget (UserInterface|GetWidget (Variables|/Script/SukProject.SukInteractionComponent|GetInteractionWidget (Variables|Default|GetInteractionComponent)))))
  (Variables|/Game/UI/WBP_InteractionWidget.WBP_InteractionWidget_C|SetInteractionText _aswbp_interaction_widget (Variables|/Script/SukProject.SukItemInstance|GetInteractText _itemcpp))
  (Components|StaticMesh|SetStaticMesh (Variables|Default|GetStaticMesh) (Variables|/Script/SukProject.SukItemInstance|GetMesh _itemcpp)))

(event Collision|EventActorBeginOverlap
  (params (OtherActor :type Actor%20Object%20Reference)))

(event EventTick
  (params (DeltaSeconds :type Float%20%28single-precision%29))
  (Transformation|AddWorldRotation (Variables|Default|GetStaticMesh) "0.000000,1.000000,0.000000" false false))

(fn ConstructionScript)