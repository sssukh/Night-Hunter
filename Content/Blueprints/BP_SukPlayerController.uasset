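; Player controller Blueprint that manages the player's character inventory as an array of item entries, each holding an item instance and quantity.
; AddItemToInventory validates the item, scans the whole array for the same instance, then overwrites that entry or appends a new one with quantity one.
; The overwrite takes its incremented quantity from the loop's element pin after completion, so from the last entry scanned rather than the match.
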(event EventBeginPlay)

(event EventTick
  (params (DeltaSeconds :type Float%20%28single-precision%29)))

(fn ConstructionScript)

(fn AddItemtoInventory
  (params (Item :type Suk%20Item%20Instance%20Object%20Reference))
  (bind _characterinventory (Variables|Default|GetCharacterInventory))
  (bind _returnvalue (Utilities|Array|Length _characterinventory))
  ;[1 1 1] Add Item To Inventory
  (Utilities|IsValid Item
    (:Is%20Valid
      (Variables|Default|SetItemIndex _returnvalue)
      (for (_array_element _array_index) _characterinventory
        (if (== Item (.ItemInstance (Utilities|Struct|BreakItemEntry _array_element)))
          (Variables|Default|SetItemIndex _array_index)))
      (if (< (Variables|Default|GetItemIndex) _returnvalue)
        (Utilities|Array|SetArrayElem _characterinventory (Variables|Default|GetItemIndex) (Utilities|Struct|MakeItemEntry Item (+ (.qty (Utilities|Struct|BreakItemEntry _array_element)) 1)))
        (else
          (Utilities|Array|Add (Variables|Default|GetCharacterInventory) (Utilities|Struct|MakeItemEntry Item 1)))))))